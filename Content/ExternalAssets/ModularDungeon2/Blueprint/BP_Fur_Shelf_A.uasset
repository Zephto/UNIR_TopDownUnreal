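; Modular dungeon bookshelf prop that varies its book arrangement through randomization in the construction script.
; It splits twelve book components into three groups of four and hides one random pick from each, along with its children.
; It then nudges the book components along local Y by a small random amount.
; The event graph has no active logic.
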(fn `UserConstructionScript`
  (bind _props_books_a (`self.Props_Books_A`))
  (`SceneComponent.SetVisibility` (select `int` (`KismetMathLibrary.RandomIntegerInRange` 0 3) :`0` _props_books_a :`1` (`self.Props_Books_B4`) :`2` (`self.Props_Books_B`) :`3` (`self.Props_Books_C`)) false true)
  (`SceneComponent.SetVisibility` (select `int` (`KismetMathLibrary.RandomIntegerInRange` 0 3) :`0` (`self.Props_Books_A3`) :`1` (`self.Props_Books_C2`) :`2` (`self.Props_Books_B3`) :`3` (`self.Props_Books_B2`)) false true)
  (`SceneComponent.SetVisibility` (select `int` (`KismetMathLibrary.RandomIntegerInRange` 0 3) :`0` (`self.Props_Books_A2`) :`1` (`self.Props_Books_B1`) :`2` (`self.Props_Books_A4`) :`3` (`self.Props_Books_C1`)) false true)
  (`SceneComponent.K2_AddLocalTransform` _props_books_a (`KismetMathLibrary.MakeTransform` (`KismetMathLibrary.MakeVector` 0.0 (`KismetMathLibrary.RandomFloatInRange` -5.0 5.0))) false false)
  (`SceneComponent.K2_AddLocalTransform` (`self.Props_Books_B4`) (`KismetMathLibrary.MakeTransform` (`KismetMathLibrary.MakeVector` 0.0 (`KismetMathLibrary.RandomFloatInRange` -5.0 5.0))) false false)
  (`SceneComponent.K2_AddLocalTransform` (`self.Props_Books_B`) (`KismetMathLibrary.MakeTransform` (`KismetMathLibrary.MakeVector` 0.0 (`KismetMathLibrary.RandomFloatInRange` -5.0 5.0))) false false)
  (`SceneComponent.K2_AddLocalTransform` (`self.Props_Books_C`) (`KismetMathLibrary.MakeTransform` (`KismetMathLibrary.MakeVector` 0.0 (`KismetMathLibrary.RandomFloatInRange` -5.0 5.0))) false false)
  (`SceneComponent.K2_AddLocalTransform` (`self.Props_Books_A3`) (`KismetMathLibrary.MakeTransform` (`KismetMathLibrary.MakeVector` 0.0 (`KismetMathLibrary.RandomFloatInRange` -5.0 5.0))) false false)
  (`SceneComponent.K2_AddLocalTransform` (`self.Props_Books_C2`) (`KismetMathLibrary.MakeTransform` (`KismetMathLibrary.MakeVector` 0.0 (`KismetMathLibrary.RandomFloatInRange` -5.0 5.0))) false false)
  (`SceneComponent.K2_AddLocalTransform` (`self.Props_Books_B3`) (`KismetMathLibrary.MakeTransform` (`KismetMathLibrary.MakeVector` 0.0 (`KismetMathLibrary.RandomFloatInRange` -5.0 5.0))) false false)
  (`SceneComponent.K2_AddLocalTransform` (`self.Props_Books_B2`) (`KismetMathLibrary.MakeTransform` (`KismetMathLibrary.MakeVector` 0.0 (`KismetMathLibrary.RandomFloatInRange` -5.0 5.0))) false false)
  (`SceneComponent.K2_AddLocalTransform` (`self.Props_Books_A2`) (`KismetMathLibrary.MakeTransform` (`KismetMathLibrary.MakeVector` 0.0 (`KismetMathLibrary.RandomFloatInRange` -5.0 5.0))) false false)
  (`SceneComponent.K2_AddLocalTransform` (`self.Props_Books_B1`) (`KismetMathLibrary.MakeTransform` (`KismetMathLibrary.MakeVector` 0.0 (`KismetMathLibrary.RandomFloatInRange` -5.0 5.0))) false false)
  (`SceneComponent.K2_AddLocalTransform` (`self.Props_Books_A4`) (`KismetMathLibrary.MakeTransform` (`KismetMathLibrary.MakeVector` 0.0 (`KismetMathLibrary.RandomFloatInRange` -5.0 5.0))) false false)
  (`SceneComponent.K2_AddLocalTransform` (`self.Props_Books_C1`) (`KismetMathLibrary.MakeTransform` (`KismetMathLibrary.MakeVector` 0.0 (`KismetMathLibrary.RandomFloatInRange` -5.0 5.0))) false false))
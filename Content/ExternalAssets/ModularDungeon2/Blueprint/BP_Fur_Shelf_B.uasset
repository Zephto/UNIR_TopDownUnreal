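; Modular dungeon shelf prop that randomizes its pottery dressing in the Construction Script.
; Nine pottery components are split into three groups of three, and a random Select per group hides one piece along with its children.
; All nine are then nudged by a small random local Y offset to vary placement.
; The Event Graph holds no active logic.
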(fn `UserConstructionScript`
  (bind _props_pottery_f (`self.Props_Pottery_F`))
  (`SceneComponent.SetVisibility` (select `int` (`KismetMathLibrary.RandomIntegerInRange` 0 2) :`0` _props_pottery_f :`1` (`self.Props_Pottery_A`) :`2` (`self.Props_Pottery_D`)) false true)
  (`SceneComponent.SetVisibility` (select `int` (`KismetMathLibrary.RandomIntegerInRange` 0 2) :`0` (`self.Props_Pottery_B2`) :`1` (`self.Props_Pottery_B1`) :`2` (`self.Props_Pottery_E`)) false true)
  (`SceneComponent.SetVisibility` (select `int` (`KismetMathLibrary.RandomIntegerInRange` 0 2) :`0` (`self.Props_Pottery_B`) :`1` (`self.Props_Pottery_C`) :`2` (`self.Props_Pottery_C1`)) false true)
  (`SceneComponent.K2_AddLocalTransform` _props_pottery_f (`KismetMathLibrary.MakeTransform` (`KismetMathLibrary.MakeVector` 0.0 (`KismetMathLibrary.RandomFloatInRange` -5.0 5.0))) false false)
  (`SceneComponent.K2_AddLocalTransform` (`self.Props_Pottery_A`) (`KismetMathLibrary.MakeTransform` (`KismetMathLibrary.MakeVector` 0.0 (`KismetMathLibrary.RandomFloatInRange` -5.0 5.0))) false false)
  (`SceneComponent.K2_AddLocalTransform` (`self.Props_Pottery_D`) (`KismetMathLibrary.MakeTransform` (`KismetMathLibrary.MakeVector` 0.0 (`KismetMathLibrary.RandomFloatInRange` -5.0 5.0))) false false)
  (`SceneComponent.K2_AddLocalTransform` (`self.Props_Pottery_E`) (`KismetMathLibrary.MakeTransform` (`KismetMathLibrary.MakeVector` 0.0 (`KismetMathLibrary.RandomFloatInRange` -5.0 5.0))) false false)
  (`SceneComponent.K2_AddLocalTransform` (`self.Props_Pottery_B`) (`KismetMathLibrary.MakeTransform` (`KismetMathLibrary.MakeVector` 0.0 (`KismetMathLibrary.RandomFloatInRange` -5.0 5.0))) false false)
  (`SceneComponent.K2_AddLocalTransform` (`self.Props_Pottery_C`) (`KismetMathLibrary.MakeTransform` (`KismetMathLibrary.MakeVector` 0.0 (`KismetMathLibrary.RandomFloatInRange` -5.0 5.0))) false false)
  (`SceneComponent.K2_AddLocalTransform` (`self.Props_Pottery_B2`) (`KismetMathLibrary.MakeTransform` (`KismetMathLibrary.MakeVector` 0.0 (`KismetMathLibrary.RandomFloatInRange` -5.0 5.0))) false false)
  (`SceneComponent.K2_AddLocalTransform` (`self.Props_Pottery_C1`) (`KismetMathLibrary.MakeTransform` (`KismetMathLibrary.MakeVector` 0.0 (`KismetMathLibrary.RandomFloatInRange` -5.0 5.0))) false false)
  (`SceneComponent.K2_AddLocalTransform` (`self.Props_Pottery_B1`) (`KismetMathLibrary.MakeTransform` (`KismetMathLibrary.MakeVector` 0.0 (`KismetMathLibrary.RandomFloatInRange` -5.0 5.0))) false false))